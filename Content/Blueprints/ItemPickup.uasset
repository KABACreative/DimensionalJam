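; Item pickup actor that lets the player take one item and put it back in its matching space, using E.
; BeginPlay and the E logic read mesh and material from Item_DT by ItemName, or the EMPTY row once taken.
; The held item lives in SharedGameInstance.CurrentItem, so an item already held leaves its mesh unset on BeginPlay.
; Overlap begin and end toggle input on the overlapping TEMP_PC.
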(event Collision|EventActorBeginOverlap
  (params (OtherActor :type Actor%20Object%20Reference))
  ;[1 1 1] Enable input when in range
  (bind _astemp_pc (Utilities|Casting|CastToTEMP_PC OtherActor))
  (Input|EnableInput _astemp_pc (Game|GetPlayerController 0)))

(event Collision|EventActorEndOverlap
  (params (OtherActor :type Actor%20Object%20Reference))
  ;[1 1 1] Disable input when out of range
  (bind _astemp_pc (Utilities|Casting|CastToTEMP_PC OtherActor))
  (Input|DisableInput _astemp_pc (Game|GetPlayerController 0)))

(event EventBeginPlay
  (bind _staticmesh (Variables|Default|GetStaticMesh))
  ;[1 0.04928 0.119] Set instance variable BROKEN - Katya
  (bind _asshared_game_instance (Utilities|Casting|CastToSharedGameInstance (Game|GetGameInstance)))
  (Variables|Default|SetSharedGameInstance _asshared_game_instance)
  (Development|PrintString "GameInstanceSet")
  ;[1 1 1] What item is this?
  (bind _returnvalue (Utilities|GetDataTableRow "/Game/Blueprints/Item_DT.Item_DT" (Variables|Default|GetItemName))
    (:then
      (bind _output_get (Variables|Default|SetItem# (.Item (Utilities|Struct|BreakItem_Struct _returnvalue))))
      ;[1 1 1] Should this be empty?
      (if (== _output_get (Variables|/Game/Blueprints/SharedGameInstance.SharedGameInstance_C|GetCurrentItem# (Variables|Default|GetSharedGameInstance)))
        (Development|PrintString "EmptySpace")
        (else
          ;[1 1 1] Set item
          (Components|StaticMesh|SetStaticMesh _staticmesh (.StaticMesh (Utilities|Struct|BreakItem_Struct _returnvalue)))
          (Rendering|Material|SetMaterial _staticmesh 0 (.Material (Utilities|Struct|BreakItem_Struct _returnvalue))))))))

(event Input|KeyboardEvents|E
  (params (Key :type Key%20Structure :default "None"))
  (bind _staticmesh (Variables|Default|GetStaticMesh))
  (bind _staticmesh_2 (Variables|Default|GetStaticMesh))
  ;[1 1 1] ItemPickup
  (:Pressed
    (bind _asshared_game_instance (Utilities|Casting|CastToSharedGameInstance (Game|GetGameInstance)))
    (if (== (Variables|/Game/Blueprints/SharedGameInstance.SharedGameInstance_C|GetCurrentItem# _asshared_game_instance) 0)
      (bind _output_get (Variables|/Game/Blueprints/SharedGameInstance.SharedGameInstance_C|SetCurrentItem# (Variables|Default|GetSharedGameInstance) (Variables|Default|GetItem#)))
      (Development|PrintString (Utilities|String|ToString(Integer) _output_get))
      (Variables|/Game/Blueprints/SharedGameInstance.SharedGameInstance_C|SetCurrentItem# (Variables|Default|GetSharedGameInstance) (Variables|Default|GetItem#))
      ;[1 1 1] CreateEmptySpace
      (bind _returnvalue (Utilities|GetDataTableRow "/Game/Blueprints/Item_DT.Item_DT" "EMPTY")
        (:then
          (Components|StaticMesh|SetStaticMesh _staticmesh (.StaticMesh (Utilities|Struct|BreakItem_Struct _returnvalue)))
          (Rendering|Material|SetMaterial _staticmesh 0 (.Material (Utilities|Struct|BreakItem_Struct _returnvalue)))))
      (else
        ;[1 1 1] Does the current item match the space?
        (if (== (Variables|/Game/Blueprints/SharedGameInstance.SharedGameInstance_C|GetCurrentItem# _asshared_game_instance) (Variables|Default|GetItem#))
          ;[1 1 1] ReplaceObject
          (bind _returnvalue_2 (Utilities|GetDataTableRow "/Game/Blueprints/Item_DT.Item_DT" (Variables|Default|GetItemName))
            (:then
              (Components|StaticMesh|SetStaticMesh _staticmesh_2 (.StaticMesh (Utilities|Struct|BreakItem_Struct _returnvalue_2)))
              (Rendering|Material|SetMaterial _staticmesh_2 0 (.Material (Utilities|Struct|BreakItem_Struct _returnvalue_2)))
              (Variables|/Game/Blueprints/SharedGameInstance.SharedGameInstance_C|SetCurrentItem# (Variables|Default|GetSharedGameInstance) 0)))
          (else
            (Development|PrintString "Your hands are full!")))))))

(fn ConstructionScript)